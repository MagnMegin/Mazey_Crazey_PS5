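; BP_MapSystem shows a map widget on screen while the MazeyMan player character stands still.
; On BeginPlay it creates the widget, passes it a texture, adds it to the viewport and caches the controlled pawn.
; Each tick it makes the map visible only when MapActive is set and both move input and velocity are near zero, hiding it otherwise.
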(event EventBeginPlay
  (bind _returnvalue (UserInterface|CreateWidget "/Game/UI/MapWidget.MapWidget_C"))
  (bind _output_get (Variables|Default|SetMapWidget _returnvalue))
  (Variables|/Game/UI/MapWidget.MapWidget_C|SetTexture _output_get (Variables|Default|GetTexture))
  (UserInterface|Viewport|AddtoViewport (Variables|Default|GetMapWidget) 0)
  (CallFunction|SetActive (Variables|Default|GetMap_Active))
  (bind _asmazey_man (Utilities|Casting|CastToMazeyMan (Pawn|GetControlledPawn (Game|GetPlayerController 0))))
  (Variables|Default|SetPlayerCharacter _asmazey_man))

(event EventTick
  (params (DeltaSeconds :type Float%20%28single-precision%29))
  (bind _playercharacter (Variables|Default|GetPlayerCharacter))
  (CallFunction|SetActive (Math|Boolean|ANDBoolean (< (Math|Vector|VectorLength (Default|GetMoveInput _playercharacter)) 0.1) (< (Math|Vector|VectorLength (Transformation|GetVelocity _playercharacter)) 1e+02) (Variables|Default|GetMap_Active))))

(fn ConstructionScript)

(fn SetActive
  (params (IsActive :type Boolean))
  (if IsActive
    (Widget|SetVisibility (Variables|Default|GetMapWidget) "Visible")
    (else
      (Widget|SetVisibility (Variables|Default|GetMapWidget) "Hidden"))))