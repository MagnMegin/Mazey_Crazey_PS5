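; Blueprint that plays a collision sound when its OnHit event fires.
; A DoOnce gate limits playback, and a delay of SoundCooldown then calls ResetSound to reopen it.
; RandomPitch appears unfinished: it only returns a neutral pitch when PitchVariability is at most one, its random-range node is unused, and playback never calls it.
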(event Custom|Event%20On%20Hit
  (Utilities|FlowControl|DoOnce false
    (:Completed
      (Audio|PlaySoundatLocation (Variables|Default|GetCollisionSound) "0, 0, 0" "0, 0, 0" 1.0 1.0 0.0 0 0 0 0)
      ;[1 1 1] Cooldown
      (Utilities|FlowControl|Delay (Variables|Default|GetSoundCooldown))
      (CallFunction|ResetSound))))

(event Custom|ResetSound
  (Utilities|FlowControl|DoOnce false) ; enters at Reset
)

(fn RandomPitch
  (if (not (> (Variables|Default|GetPitchVariability) 1.0))
    (return 1.0)))