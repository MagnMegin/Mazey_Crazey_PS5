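; BP_GameManager coordinates the rain, timer and map systems for a maze section of the game.
; On BeginPlay, Instantiate finds the placed BP_RainSystem, BP_TimerSystem and BP_MapSystem actors by class, caches them, and prints a red warning for any missing one.
; StartMaze starts the rain and timer and activates the map; EndMaze pauses both and deactivates the map.
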(event EventBeginPlay
  (CallFunction|Instantiate))

(fn ConstructionScript)

(fn Instantiate
  (bind _returnvalue (Actor|GetActorOfClass "/Game/Blueprints/BP_RainSystem.BP_RainSystem_C"))
  (bind _output_get (Variables|Default|SetRainSystem _returnvalue))
  (Utilities|IsValid _output_get
    (:Is%20Valid
      _)
    (:Is%20Not%20Valid
      (Development|PrintString "Rain system not found" true true "(R=1.000000,G=0.000000,B=0.011234,A=1.000000)")))
  (bind _returnvalue_2 (Actor|GetActorOfClass "/Game/Blueprints/BP_TimerSystem.BP_TimerSystem_C"))
  (bind _output_get_2 (Variables|Default|SetTimerSystem _returnvalue_2))
  (Utilities|IsValid _output_get_2
    (:Is%20Valid
      _)
    (:Is%20Not%20Valid
      (Development|PrintString "Timer system not found" true true "(R=1.000000,G=0.000000,B=0.011234,A=1.000000)")))
  (bind _returnvalue_3 (Actor|GetActorOfClass "/Game/Blueprints/BP_MapSystem.BP_MapSystem_C"))
  (bind _output_get_3 (Variables|Default|SetMapSystem _returnvalue_3))
  (Utilities|IsValid _output_get_3
    (:Is%20Not%20Valid
      (Development|PrintString "Map system not found" true true "(R=1.000000,G=0.000000,B=0.011234,A=1.000000)"))))

(fn StartMaze
  (Default|StartRain (Variables|Default|GetRainSystem))
  (Default|StartTimer (Variables|Default|GetTimerSystem))
  (Variables|/Game/Blueprints/BP_MapSystem.BP_MapSystem_C|SetMap_Active (Variables|Default|GetMapSystem) true))

(fn EndMaze
  (Default|PauseRain (Variables|Default|GetRainSystem))
  (Default|PauseTimer (Variables|Default|GetTimerSystem))
  (Variables|/Game/Blueprints/BP_MapSystem.BP_MapSystem_C|SetMap_Active (Variables|Default|GetMapSystem) false))