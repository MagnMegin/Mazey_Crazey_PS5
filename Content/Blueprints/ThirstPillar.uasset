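; ThirstPillar is a one-use pickup that changes a MazeyMan's thirst.
; Tick spins the Pickup component and plays a timeline that offsets its height from the position saved at BeginPlay.
; When MazeyMan first overlaps OverlapBox, it calls IncreaseThirst with IncreaseAmount, hides the Pickup and clears IsUnused, so the actor stays but cannot trigger again.
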(event OnComponentBeginOverlap(OverlapBox)
  (params (OverlappedComponent :type Primitive%20Component%20Object%20Reference) (OtherActor :type Actor%20Object%20Reference) (OtherComp :type Primitive%20Component%20Object%20Reference) (OtherBodyIndex :type Integer) (bFromSweep :type Boolean) (SweepResult :type Hit%20Result%20Structure%20%28by%20ref%29))
  (bind _asmazey_man (Utilities|Casting|CastToMazeyMan OtherActor))
  (if (Variables|Default|GetIsUnused)
    (Default|IncreaseThirst _asmazey_man (Variables|Default|GetIncreaseAmount))
    (Development|SetHiddeninGame (Variables|Default|GetPickup) true true)
    (Variables|Default|SetIsUnused false)))

(event EventTick
  (params (DeltaSeconds :type Float%20%28single-precision%29))
  (Transformation|AddLocalRotation (Variables|Default|GetPickup) (Math|Rotator|MakeRotator 0.0 0.0 (* DeltaSeconds (Variables|Default|GetRotationSpeed))) false false)
  (bind _heightoffset (Timeline|Timeline Play)
    (:Update
      (Transformation|SetWorldLocation (Variables|Default|GetPickup) (+ (Math|Vector|MakeVector 0.0 0.0 _heightoffset) (Variables|Default|GetStartPosition)) false false))))

(event EventBeginPlay
  (Variables|Default|SetStartPosition (Transformation|GetWorldLocation (Variables|Default|GetPickup))))

(fn ConstructionScript)