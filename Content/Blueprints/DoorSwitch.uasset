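; DoorSwitch is a floor or trigger switch that signals a BP_SwitchSystem when the MazeyMan character overlaps it.
; On BeginPlay it finds the switch system in the level and prints a warning if none exists.
; An overlap by MazeyMan swaps the status cube to the on material and sends the switch signal to that system.
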(event OnComponentBeginOverlap(OverlapBox)
  (params (OverlappedComponent :type Primitive%20Component%20Object%20Reference) (OtherActor :type Actor%20Object%20Reference) (OtherComp :type Primitive%20Component%20Object%20Reference) (OtherBodyIndex :type Integer) (bFromSweep :type Boolean) (SweepResult :type Hit%20Result%20Structure%20%28by%20ref%29))
  (Utilities|Casting|CastToMazeyMan OtherActor)
  (Rendering|Material|SetMaterial (Variables|Default|GetStatusCube) 0 (Variables|Default|GetOnMaterial))
  (Default|EventSendSwitchSignal (Variables|Default|GetSwitchSystem)))

(event EventBeginPlay
  (bind _returnvalue (Actor|GetActorOfClass "/Game/Blueprints/BP_SwitchSystem.BP_SwitchSystem_C"))
  (bind _output_get (Variables|Default|SetSwitchSystem _returnvalue))
  (Utilities|IsValid _output_get
    (:Is%20Not%20Valid
      (Development|PrintString "Could not find switch system" true true "(R=1.000000,G=0.000000,B=0.018970,A=1.000000)"))))

(fn ConstructionScript)