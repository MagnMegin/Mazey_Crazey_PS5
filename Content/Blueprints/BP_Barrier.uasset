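; BP_Barrier is a trigger volume that marks a maze boundary as either an entry or an exit.
; On BeginPlay it looks up BP_GameManager, caches it, and prints an error if none is found.
; When MazeyMan overlaps its Box, it tells the GameManager to start or end the maze according to its Mode.
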(event OnComponentBeginOverlap(Box)
  (params (OverlappedComponent :type Primitive%20Component%20Object%20Reference) (OtherActor :type Actor%20Object%20Reference) (OtherComp :type Primitive%20Component%20Object%20Reference) (OtherBodyIndex :type Integer) (bFromSweep :type Boolean) (SweepResult :type Hit%20Result%20Structure%20%28by%20ref%29))
  (Utilities|Casting|CastToMazeyMan OtherActor)
  (Development|PrintString "HitBarrier")
  (switch Utilities|FlowControl|Switch|SwitchonBarrierMode (Variables|Default|GetMode)
    (:NewEnumerator0
      (Default|StartMaze (Variables|Default|GetGameManager)))
    (:NewEnumerator1
      (Default|EndMaze (Variables|Default|GetGameManager)))))

(event EventBeginPlay
  (bind _returnvalue (Actor|GetActorOfClass "/Game/Blueprints/BP_GameManager.BP_GameManager_C"))
  (bind _output_get (Variables|Default|SetGameManager _returnvalue))
  (Utilities|IsValid _output_get
    (:Is%20Not%20Valid
      (Development|PrintString "Cannot find GameManager" true true "(R=1.000000,G=0.032280,B=0.000000,A=1.000000)"))))

(fn ConstructionScript)