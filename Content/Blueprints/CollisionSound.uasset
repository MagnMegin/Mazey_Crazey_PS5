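; CollisionSound plays a positional impact sound when its OnHit event is called, provided collision sounds are enabled in MazeyInstance.
; Volume scales with impulse strength above a minimum threshold and is clamped before applying a multiplier, while pitch is randomized by a variability setting.
; A DoOnce gate throttles repeated hits, resetting after a cooldown delay scaled by the game instance's multiplier.
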(event Custom|Event%20On%20Hit
  (params (HitLocation :type Vector) (HitImpulse :type Vector))
  (Utilities|IfCollisionSoundsEnabled
    (:True
      (Utilities|FlowControl|DoOnce false
        (:Completed
          (Audio|PlaySoundatLocation (Variables|Default|GetCollisionSound) HitLocation "0, 0, 0" (CallFunction|VolumefromImpulse HitImpulse) (CallFunction|RandomPitch) 0.0 (Variables|Default|GetAttenuation%20Settings) 0 0 0)
          ;[1 1 1] Cooldown
          (Utilities|FlowControl|Delay (* (Variables|Default|GetSoundCooldown) (Default|GetCooldownMultiplier (Variables|Default|GetGameInstance))))
          (CallFunction|ResetSound))))))

(event Custom|ResetSound
  (Utilities|FlowControl|DoOnce false) ; enters at Reset
)

(event EventBeginPlay
  (bind _asmazey_instance (Utilities|Casting|CastToMazeyInstance (Game|GetGameInstance))
    (:then
      (Variables|Default|SetGameInstance _asmazey_instance))
    (:CastFailed
      (Development|PrintString "Cannot find MazyeInstance" true true "(R=1.000000,G=0.000000,B=0.197837,A=1.000000)"))))

(fn RandomPitch
  (bind _pitchvariability (Variables|Default|GetPitchVariability))
  (bind _returnvalue (+ _pitchvariability 1.0))
  (if (> (Variables|Default|GetPitchVariability) 0.0)
    (return (* (Math|Random|RandomFloatinRange (/ 1.0 _returnvalue) _returnvalue) (Variables|Default|GetPitchMultiplier)))
    (else
      (return 1.0))))

(fn VolumefromImpulse
  (params (Impulse :type Vector))
  (return (* (Math|Float|Clamp(Float) (/ (- (Math|Vector|VectorLength Impulse) 3.5e+03) 1e+04)) (Variables|Default|GetVolumeMultiplier))))