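; Rain system actor that continuously spawns a configurable object at random points across an area while raining is active.
; Tick accumulates SpawnRate times delta time, spawns the whole number of queued objects and carries the fraction over, keeping the rate frame-independent.
; Spawn points lie on a flat rectangle around the actor, sized by its scale; the SpawnArea component is hidden at BeginPlay.
; StartRain and PauseRain toggle spawning, with RainOnStart setting the initial state.
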(event EventBeginPlay
  (Rendering|SetVisibility (Variables|Default|GetSpawnArea) false false)
  (Variables|Default|SetIsRaining (Variables|Default|GetRainOnStart)))

(event EventTick
  (params (DeltaSeconds :type Float%20%28single-precision%29))
  (if (Variables|Default|GetIsRaining)
    (bind _output_get (Variables|Default|SetQueuedSpawns (+ (* DeltaSeconds (Variables|Default|GetSpawnRate)) (Variables|Default|GetQueuedSpawns))))
    (bind _output_get_2 (Variables|Default|SetWholeQueuedSpawns (Math|Float|Floor _output_get)))
    (for _index (range 0 (- _output_get_2 (Class|KismetSystemLibrary|MakeLiteralInteger 1)))
      (CallFunction|SpawnObjectinRandomLocation (Variables|Default|GetSpawnObject)))
    (Variables|Default|SetQueuedSpawns (- (Variables|Default|GetQueuedSpawns) (Variables|Default|GetWholeQueuedSpawns)))))

(fn ConstructionScript)

(fn RandomSpawnPoint
  (bind _scale (CallFunction|GetActorScale))
  (return (+ (Math|Vector|MakeVector (* (Math|Random|RandomFloatinRange -5e+01 5e+01) (.x _scale)) (* (.y _scale) (Math|Random|RandomFloatinRange -5e+01 5e+01)) 0.0) (Transformation|GetActorLocation))))

(fn GetActorScale
  (return (.Scale (Math|Transform|BreakTransform (Transformation|GetActorTransform)))))

(fn SpawnObjectinRandomLocation
  (params (Class :type Actor%20Class%20Reference))
  (Game|SpawnActorfromClass Class (Math|Transform|MakeTransform (CallFunction|RandomSpawnPoint) "0, 0, 0" (Math|Conversions|ToVector(Float) (Variables|Default|GetSpawnScale))) "AdjustIfPossibleButAlwaysSpawn" 0 0))

(fn StartRain
  (Variables|Default|SetIsRaining true))

(fn PauseRain
  (Variables|Default|SetIsRaining false))