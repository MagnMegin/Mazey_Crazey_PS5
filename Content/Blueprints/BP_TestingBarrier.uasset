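; BP_TestingBarrier is a barrier actor with a trigger box that starts rain when MazeyMan overlaps it.
; The overlap prints a debug string and switches on Mode, though both Entry and Exit currently call StartRain on RainSystem.
; SetImpassible, applied on BeginPlay from StartImpassible, toggles a separate blocking box's collision and swaps the plane's material to show whether the barrier is passable.
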(event OnComponentBeginOverlap(Box)
  (params (OverlappedComponent :type Primitive%20Component%20Object%20Reference) (OtherActor :type Actor%20Object%20Reference) (OtherComp :type Primitive%20Component%20Object%20Reference) (OtherBodyIndex :type Integer) (bFromSweep :type Boolean) (SweepResult :type Hit%20Result%20Structure%20%28by%20ref%29))
  (Utilities|Casting|CastToMazeyMan OtherActor)
  (Development|PrintString "HitBarrier")
  (switch Utilities|FlowControl|Switch|SwitchonBarrierMode (Variables|Default|GetMode)
    (:NewEnumerator0
      (Default|StartRain (Variables|Default|GetRainSystem)))
    (:NewEnumerator1
      (Default|StartRain (Variables|Default|GetRainSystem)))))

(event EventBeginPlay
  (CallFunction|SetImpassible (Variables|Default|GetStartImpassible)))

(fn ConstructionScript)

(fn SetImpassible
  (params (Bool :type Boolean))
  (if Bool
    (Collision|SetCollisionEnabled (Variables|Default|GetImpassableBox) "QueryAndPhysics")
    (Rendering|Material|SetMaterial (Variables|Default|GetPlane) 0 (Variables|Default|GetImpassibleMat))
    (else
      (Collision|SetCollisionEnabled (Variables|Default|GetImpassableBox) "NoCollision")
      (Rendering|Material|SetMaterial (Variables|Default|GetPlane) 0 (Variables|Default|GetNormalMat)))))