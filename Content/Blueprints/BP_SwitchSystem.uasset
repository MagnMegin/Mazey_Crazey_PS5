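; Switch manager Blueprint that opens a door once enough switch signals arrive.
; On BeginPlay it counts every DoorSwitch actor in the level.
; Each SendSwitchSignal call increments an on-switch counter and makes DoorToOpen passable when it reaches that count.
; The counter only increases, so switches are never counted as turned off.
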(event Custom|Event%20Send%20Switch%20Signal
  (bind _result (Math|Integer|IncrementInt (Variables|Default|GetSwitchesOn))
    (:%20%20
      (if (>= _result (Variables|Default|GetSwitchCount))
        (Default|SetImpassible (Variables|Default|GetDoorToOpen) false)))))

(event EventBeginPlay
  (bind _outactors (Actor|GetAllActorsOfClass "/Game/Blueprints/DoorSwitch.DoorSwitch_C"))
  (Variables|Default|SetSwitchCount (Utilities|Array|Length _outactors)))

(fn ConstructionScript)