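; MazeyInstance, apparently the game instance, holds player survival stats and global settings as shared state.
; SaveStats stores health, hunger and thirst and raises a saved flag, which HasSavedStats reports, while LoadStats returns the values and ResetStoredStats clears them.
; Simple getter and setter pairs expose a rain multiplier and a toggle for collision sounds.
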(fn SaveStats
  (params (Health :type Float%20%28double-precision%29) (Hunger :type Float%20%28double-precision%29) (Thirst :type Float%20%28double-precision%29))
  (Variables|Default|SetStoredHealth Health)
  (Variables|Default|SetStoredHunger Hunger)
  (Variables|Default|SetStoredThirst Thirst)
  (Variables|Default|SetStatsSaved true))

(fn LoadStats
  (return (Variables|Default|GetStoredHealth) (Variables|Default|GetStoredHunger) (Variables|Default|GetStoredThirst)))

(fn HasSavedStats
  (return (Variables|Default|GetStatsSaved)))

(fn ResetStoredStats
  (Variables|Default|SetStoredHealth 0.0)
  (Variables|Default|SetStoredHunger 0.0)
  (Variables|Default|SetStoredThirst 0.0)
  (Variables|Default|SetStatsSaved false))

(fn GetRainMultiplier
  (return (Variables|Default|GetRainMultiplier)))

(fn SetRainMultiplier
  (params (Input :type Float%20%28double-precision%29))
  (Variables|Default|SetRainMultiplier Input))

(fn SetPlayCollisionSounds
  (params (Input :type Boolean))
  (Variables|Default|SetPlayCollisionSounds Input))

(fn GetPlayCollisionSounds
  (return (Variables|Default|GetPlayCollisionSounds)))